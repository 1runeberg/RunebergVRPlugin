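; Destructible ice tower actor that slowly bobs up and down until it is fractured.
; Tick nudges the destructible component vertically by a fixed per-frame offset, so speed depends on frame rate, while a looping timer flips the direction.
; On fracture it enables gravity on the component, plays an ice crash sound at the hit point and sets a lifespan so the actor cleans itself up.
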(event `self.ReceiveTick`
  (params (DeltaSeconds :type "Float (single-precision)"))
  (bind _destructible (`self.Destructible`))
  ;[1 1 1] Bob Up & Down
  (if (`self.BobUp`)
    (`SceneComponent.K2_AddWorldOffset` _destructible (0.0 0.0 0.25) false false)
    (else
      (`SceneComponent.K2_AddWorldOffset` _destructible (0.0 0.0 -0.25) false false))))

(event `self.ReceiveBeginPlay`
  ;[1 1 1] Bob Up & Down
  (`KismetSystemLibrary.K2_SetTimerDelegate` (delegate `Bob`) 3.0 true))

(event `Bob`
  ;[1 1 1] Bob Up & Down
  (if (`self.BobUp`)
    (set `self.BobUp` false)
    (else
      (set `self.BobUp` true))))

(event `self.Destructible.OnComponentFracture`
  (params (HitPoint :type "Vector Structure (by ref)") (HitDirection :type "Vector Structure (by ref)"))
  ;[1 1 1] Apply FX on Destruction
  (`PrimitiveComponent.SetEnableGravity` (`self.Destructible`) true)
  (`self.SetLifeSpan` 8.0)
  (`GameplayStatics.PlaySoundAtLocation` "/Game/Audio/A_Ice_Crash.A_Ice_Crash" HitPoint))

(fn `UserConstructionScript`)