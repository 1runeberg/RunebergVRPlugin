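; Surfboard actor for the VR movement map that stays beneath the player pawn's camera at a fixed Z offset.
; Each tick it takes rotation from the camera when idle or the active motion controller when moving, clamping roll and pitch.
; Overlapping an actor tagged VRBounds bounces the pawn back via RunebergVRMovement, hides both power spheres and plays a sound.
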(event `self.ReceiveBeginPlay`
  ;[1 1 1] Set the VR Pawn as a constant
  (bind _as3_movement_vrpawn (cast `/Game/Maps/3_Movement/3_Movement_VRPawn` (`Controller.K2_GetPawn` (`GameplayStatics.GetPlayerController` 0))))
  (set `self.ControllingPawn` _as3_movement_vrpawn))

(event `self.ReceiveTick`
  (params (DeltaSeconds :type "Float (single-precision)"))
  (bind _controllingpawn (`self.ControllingPawn`))
  (bind (_sourcerotation_roll _sourcerotation_pitch) (`KismetMathLibrary.BreakRotator` (`self.SourceRotation`)))
  (bind (_sourcerotation_roll_2 _sourcerotation_pitch_2 _sourcerotation_yaw) (`KismetMathLibrary.BreakRotator` (`self.SourceRotation`)))
  (bind _returnvalue (`SceneComponent.K2_GetComponentToWorld` (`RunebergVR_Pawn.Camera` (`self.ControllingPawn`))))
  (`|ExecutionSequence`
    (:`then_0`
      ;[1 1 1] Set rotation source (Camera if moving, active controller otherwise)
      (if (not (`RunebergVR_Movement.IsMoving` (`/Game/Maps/3_Movement/3_Movement_VRPawn.RunebergVR_Movement` _controllingpawn)))
        (set `self.SourceRotation` (`SceneComponent.RelativeRotation` (`RunebergVR_Pawn.Camera` _controllingpawn)))
        (elif (`/Game/Maps/3_Movement/3_Movement_VRPawn.LeftControllerActive` _controllingpawn)
          (set `self.SourceRotation` (`SceneComponent.RelativeRotation` (`RunebergVR_Pawn.MotionController_Left` _controllingpawn)))
          (else
            (set `self.SourceRotation` (`SceneComponent.RelativeRotation` (`RunebergVR_Pawn.MotionController_Right` _controllingpawn)))))))
    (:`then_1`
      ;[1 1 1] Constrain the Roll of the surfboard to max / min 25 degrees
      (if (> _sourcerotation_roll 25.0)
        (set `self.ConstrainedRoll` 25.0)
        (elif (< _sourcerotation_roll -25.0)
          (set `self.ConstrainedRoll` -25.0)
          (else
            (set `self.ConstrainedRoll` _sourcerotation_roll)))))
    (:`then_2`
      ;[1 1 1] Constrain Pitch between -10 and +5 degrees
      (if (> _sourcerotation_pitch 5.0)
        (set `self.ConstrainedPitch` 5.0)
        (elif (< _sourcerotation_pitch -10.0)
          (set `self.ConstrainedPitch` -10.0)
          (else
            (set `self.ConstrainedPitch` _sourcerotation_pitch)))))
    (:`then_3`
      ;[1 1 1] Follow the pawn maintaining a constant Z axis offset
      (`self.K2_SetActorLocation` (`KismetMathLibrary.MakeVector` (.x (.location _returnvalue)) (.y (.location _returnvalue)) (- (.z (.location _returnvalue)) (`self.Z Offset`))))
      (`self.K2_SetActorRotation` (`KismetMathLibrary.MakeRotator` (`self.ConstrainedRoll`) (`self.ConstrainedPitch`) _sourcerotation_yaw)))))

(event `self.StaticMesh.OnComponentBeginOverlap`
  (params (OverlappedComponent :type "PrimitiveComponent Object Reference") (OtherActor :type "Actor Object Reference") (OtherComp :type "PrimitiveComponent Object Reference") (OtherBodyIndex :type Integer) (bFromSweep :type Boolean) (SweepResult :type "HitResult Structure (by ref)"))
  ;[1 0.4478 0.4578] Bounce player back if this surfboard overlaps with VR Bounds
  (if (`self.ActorHasTag` OtherActor "VRBounds")
    (bind _as3_movement_vrpawn (cast `/Game/Maps/3_Movement/3_Movement_VRPawn` (`GameplayStatics.GetPlayerPawn` 0)))
    (`RunebergVR_Movement.BounceBackFromVRBounds` (`/Game/Maps/3_Movement/3_Movement_VRPawn.RunebergVR_Movement` _as3_movement_vrpawn) 5.0 0.5 false)
    (`|ExecutionSequence`
      (:`then_0`
        (`/Game/Maps/3_Movement/3_Movement_VRPawn.PowerSphere` _as3_movement_vrpawn (`/Game/Maps/3_Movement/3_Movement_VRPawn.StaticMesh_Power_L` _as3_movement_vrpawn) false false))
      (:`then_1`
        (`/Game/Maps/3_Movement/3_Movement_VRPawn.PowerSphere` _as3_movement_vrpawn (`/Game/Maps/3_Movement/3_Movement_VRPawn.StaticMesh_Power_R` _as3_movement_vrpawn) false false)))
    (`GameplayStatics.PlaySoundAtLocation` null (`self.K2_GetActorLocation`))))

(fn `UserConstructionScript`)