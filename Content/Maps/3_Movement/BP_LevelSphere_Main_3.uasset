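; Level-switch sphere in the VR movement map that sends the player back to the 1_Main level.
; Its text label spins slightly every tick.
; When its collision sphere begins overlapping the VR pawn's capsule, it opens that level only if the actor is no more than 25 units below the pawn's camera, so it must be near head height or higher.
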(event `self.ReceiveTick`
  (params (DeltaSeconds :type "Float (single-precision)"))
  ;[1 1 1] Rotatre Text
  (`SceneComponent.K2_AddLocalRotation` (`self.TextRender`) (struct :`Yaw` 1.0) false false))

(event `self.SphereCollision.OnComponentBeginOverlap`
  (params (OverlappedComponent :type "PrimitiveComponent Object Reference") (OtherActor :type "Actor Object Reference") (OtherComp :type "PrimitiveComponent Object Reference") (OtherBodyIndex :type Integer) (bFromSweep :type Boolean) (SweepResult :type "HitResult Structure (by ref)"))
  (bind (_returnvalue_x _returnvalue_y _returnvalue_z) (`KismetMathLibrary.BreakVector` (`self.K2_GetActorLocation`)))
  ;[1 1 1] Open new level when this sphere collides with the capsule component of the VR Pawn
  (bind _as3_movement_vrpawn (cast `/Game/Maps/3_Movement/3_Movement_VRPawn` OtherActor))
  (cast `CapsuleComponent` OtherComp)
  (bind (_returnvalue_x_2 _returnvalue_y_2 _returnvalue_z_2) (`KismetMathLibrary.BreakVector` (`SceneComponent.K2_GetComponentLocation` (`RunebergVR_Pawn.Camera` _as3_movement_vrpawn))))
  (if (>= _returnvalue_z (- _returnvalue_z_2 25.0))
    (`GameplayStatics.OpenLevel` "1_Main")))

(fn `UserConstructionScript`)